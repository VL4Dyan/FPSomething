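; Team game mode that tracks players as undefined, spectators, RED or BLU and spawns team members as BP_Scout pawns.
; BeginPlay caches each team's BP_SpawnArea, and PostLogin flags the game state as started once more than one undefined player is present.
; TrySwitchPlayerTeam only moves undefined players, then calls SpawnPlayer, which spawns and possesses scouts at locations from the team's spawn area.
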(event `self.ReceiveBeginPlay`
  (bind _outactors (`GameplayStatics.GetAllActorsOfClass` "/Game/Blueprints/BP_SpawnArea.BP_SpawnArea_C"))
  (for _array_element _outactors
    (switch `ETeamAffiliation` (`/Game/Blueprints/BP_SpawnArea.TeamAffiliation` _array_element)
      (:`TeamBLU`
        (set `self.BLUSpawn` _array_element))
      (:`TeamRED`
        (set `self.REDSpawn` _array_element)))))

(event `self.K2_PostLogin`
  (params (NewPlayer :type "PlayerController Object Reference"))
  (bind _undefinedplayers (`self.UndefinedPlayers`))
  (`KismetArrayLibrary.Array_Add` _undefinedplayers NewPlayer)
  (if (> (`KismetArrayLibrary.Array_Length` _undefinedplayers) 1)
    (bind _asfpsmth_game_state_base (cast `FPSmthGameStateBase` (`GameplayStatics.GetGameState`)))
    (`FPSmthGameStateBase.SetGameStarted` _asfpsmth_game_state_base true)
    (clear `FPSmthGameStateBase.OnGameStarted` _asfpsmth_game_state_base)))

(fn `SpawnPlayer`
  (params (Player :type "Controller Object Reference"))
  (locals (PlayerVar :type "Controller Object Reference"))
  (bind _output_get (set `local.PlayerVar` Player))
  (`self.CurrentPlayerAffiliation` _output_get
    (:`RED`
      (bind _newparam (`/Game/Blueprints/BP_SpawnArea.GetSpawnLocations` (`self.REDSpawn`) 0))
      (for _array_element _newparam
        (bind _returnvalue (`|SpawnActorFromClass` "/Game/Blueprints/PlayerClasses/Scout/BP_Scout.BP_Scout_C" _array_element "AdjustIfPossibleButAlwaysSpawn" "OverrideRootScale" (`local.PlayerVar`) null))
        (`Controller.Possess` (`local.PlayerVar`) _returnvalue)))
    (:`BLU`
      (bind _newparam_2 (`/Game/Blueprints/BP_SpawnArea.GetSpawnLocations` (`self.BLUSpawn`) 0))
      (for _array_element_2 _newparam_2
        (bind _returnvalue_2 (`|SpawnActorFromClass` "/Game/Blueprints/PlayerClasses/Scout/BP_Scout.BP_Scout_C" _array_element_2 "AdjustIfPossibleButAlwaysSpawn" "OverrideRootScale" (`local.PlayerVar`) null))
        (`Controller.Possess` (`local.PlayerVar`) _returnvalue_2)))))

(fn `TrySwitchPlayerTeam`
  (params (Player :type "Controller Object Reference") (NewPlayerTeam :type "ETeamAffiliation Enum" :default "Undefined"))
  (returns (ReturnValue :type Boolean))
  (locals (Success :type Boolean))
  (`self.CurrentPlayerAffiliation` Player
    (:`Undefined`
      (switch `ETeamAffiliation` NewPlayerTeam
        (:`Undefined`
          _)
        (:`Spectators`
          (`KismetArrayLibrary.Array_AddUnique` (`self.Spectators`) Player)
          (`KismetArrayLibrary.Array_RemoveItem` (`self.UndefinedPlayers`) Player :!label _label)
          (set `local.Success` true)
          (`self.SpawnPlayer` Player))
        (:`TeamBLU`
          (`KismetArrayLibrary.Array_AddUnique` (`self.PlayersBLU`) Player)
          (goto _label))
        (:`TeamRED`
          (`KismetArrayLibrary.Array_AddUnique` (`self.PlayersRED`) Player)
          (goto _label)))
      (return (`local.Success`)))))

(fn `UserConstructionScript`)