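; Gameplay Ability that reloads the source weapon, activatable only when it is below max loaded ammo and has carried ammo.
; It caches weapon and character, then plays montages on first- and third-person meshes.
; A third-person montage event moves one round from carried to loaded and ends the ability, with WaitNetSync tasks for network synchronization.
; Montage interruption cancels it, and the ContinuousReload branch on end is empty.
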(event `self.K2_ActivateAbility`
  (bind _sourceweapon (`self.SourceWeapon`))
  (bind _sourceweapon_2 (`self.SourceWeapon`))
  (`self.CheckAndSetUpVariables`)
  (`AT_PlayMontageForMeshAndWaitForEvent.PlayMontageForMeshAndWaitForEvent` "None" (`CharacterBase.GetFirstPersonMesh` (`self.OwnerCharacter`))
    (:`then`
      (`AT_PlayMontageForMeshAndWaitForEvent.PlayMontageForMeshAndWaitForEvent` "None" (`CharacterBase.GetThirdPersonMesh` (`self.OwnerCharacter`))
        (:`OnCompleted`
          (`AbilityTask_NetworkSyncPoint.WaitNetSync` "BothWait"
            (:`OnSync`
              (`self.K2_EndAbility`))))
        (:`OnInterrupted`
          (`self.K2_CancelAbility` :!label _label))
        (:`OnCancelled`
          (goto _label))
        (:`EventReceived`
          (`AbilityTask_NetworkSyncPoint.WaitNetSync` "OnlyServerWait"
            (:`then`
              (`Weapon.SetCarriedAmmo` _sourceweapon (- (`Weapon.GetCarriedAmmo` _sourceweapon) 1))
              (`Weapon.SetLoadedAmmo` _sourceweapon_2 (+ (`Weapon.GetLoadedAmmo` _sourceweapon_2) 1))
              (`self.K2_EndAbility`))))))))

(event `self.K2_OnEndAbility`
  (params (bWasCancelled :type Boolean))
  (if bWasCancelled
    _
    (elif (`self.ContinuousReload`)
      _)))

(fn `K2_CanActivateAbility`
  (params (ActorInfo :type "GameplayAbilityActorInfo Structure"))
  (returns (RelevantTags :type "GameplayTagContainer Structure") (ReturnValue :type Boolean))
  (locals (Result :type Boolean))
  (bind _sourceweapon (`self.SourceWeapon`))
  (return (struct) (and (< (`Weapon.GetLoadedAmmo` _sourceweapon) (`Weapon.GetMaxLoadedAmmo` _sourceweapon)) (> (`Weapon.GetCarriedAmmo` _sourceweapon) 0))))