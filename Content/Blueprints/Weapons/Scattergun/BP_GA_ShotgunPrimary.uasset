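; Shotgun primary fire Gameplay Ability that drives a separate BP_GA_ShotgunPrimary_Instant ability.
; Caches the source weapon and the instant ability's handle and instance, then waits a frame for montages to stop.
; Activates the instant ability through a batched RPC, waits TimeBetweenShots, then loops Fire while the cost check passes, with no delay inside the loop.
; Input release or a failed cost check ends both abilities.
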(event `self.K2_ActivateAbility`
  (`self.CheckAndSetUpVariables`)
  (`AT_WaitDelayOneFrame.WaitDelayOneFrame` ; A delay to let currently playing montages to stop
    (:`OnFinish`
      (bind _returnvalue (`self.BatchRPCTryActivateAbility` (`self.InstantAbilityHandle`)))
      (if _returnvalue
        (`AbilityTask_WaitInputRelease.WaitInputRelease` true
          (:`then`
            (`AbilityTask_WaitDelay.WaitDelay` (`self.TimeBetweenShots`)
              (:`OnFinish`
                (bind _returnvalue_2 (`self.K2_CheckAbilityCost` :!label _label))
                (if _returnvalue_2
                  (`/Game/Blueprints/Weapons/Scattergun/BP_GA_ShotgunPrimary_Instant.Fire` (`self.InstantAbility`))
                  (goto _label)
                  (else
                    _)))))
          (:`OnRelease`
            _))
        (`self.K2_EndAbility` (`self.InstantAbility`))
        (`self.K2_EndAbility`)
        (else
          (`self.K2_EndAbility`))))))