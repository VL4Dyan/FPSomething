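; Gameplay ability that fires one instant scattergun shot, paced by the fire interval of BP_GA_ShotgunPrimary.
; The local controller runs a reusable multi-pellet line trace with spread, configured with the muzzle socket and player-viewpoint aiming.
; Server and client share a target data handler that commits cost, plays the montage, applies SetByCaller pellet damage and fires the gameplay cue.
; The server receives client target data through a wait task, ended with the ability.
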(event `self.K2_ActivateAbility`
  (`self.CheckAndSetUpVariables`)
  (bind (_asynctaskproxy _data) (`AT_ServerWaitForClientTargetData.ServerWaitForClientTargetData` "None")
    (:`then`
      (set `self.ServerWaitTargetDataTask` _asynctaskproxy)
      (`self.Fire`))
    (:`ValidData`
      (`self.HandleTargetData` _data))))

(event `Fire`
  (if (`Controller.IsLocalPlayerController` (`.PlayerController` (break `GameplayAbilityActorInfo` (`self.GetActorInfo`))))
    (if (>= (`KismetMathLibrary.Abs` (- (`GameplayStatics.GetTimeSeconds`) (`self.TimeOfLastShot`))) (- (`/Game/Blueprints/Weapons/Scattergun/BP_GA_ShotgunPrimary.TimeBetweenShots` (`self.GA_Primary`)) 0.01))
      (bind _returnvalue (`self.K2_CheckAbilityCost`))
      (if _returnvalue
        (`/Engine/EditorBlueprintResources/StandardMacros.IsValid` (`self.SourceWeapon`)
          (:`Is Valid`
            (set `self.TraceStartLocation` (make `GameplayAbilityTargetingLocationInfo` "SocketTransform" "0.000000,0.000000,0.000000|0.000000,0.000000,0.000000|1.000000,1.000000,1.000000" null (`self.FPWeaponMesh`) null "Muzzle"))
            (`GATA_LineTrace.Configure` :`self` (`self.LineTraceTargetActor`) :`InStartLocation` (`self.TraceStartLocation`) :`InTraceProfile` (struct :`Name` "Projectile") :`bInTraceFromPlayerViewPoint` true :`InBaseSpread` (`self.WeaponSpread`) :`InNumberOfTraces` (`self.NumberOfPellets`))
            (bind (_asynctaskproxy _data) (`AT_WaitTargetDataUsingActor.WaitTargetDataWithReusableActor` "None" "Instant" null true)
              (:`then`
                (set `self.TimeOfLastShot` (`GameplayStatics.GetTimeSeconds`)))
              (:`ValidData`
                (`self.HandleTargetData` _data)))))
        (else
          (`self.K2_CancelAbility`))))))

(event `HandleTargetData`
  (params (TargetData :type "GameplayAbilityTargetDataHandle Structure"))
  (bind _returnvalue (`self.K2_CommitAbilityCost` false))
  (if _returnvalue
    (`self.PlayMontage`)
    (bind _returnvalue_2 (`AbilitySystemBlueprintLibrary.AssignTagSetByCallerMagnitude` (`self.MakeOutgoingGameplayEffectSpec` null) (struct :`TagName` "Data.Damage") (`self.PelletDamage`)))
    (`self.K2_ApplyGameplayEffectSpecToTarget` _returnvalue_2 TargetData)
    (bind _returnvalue_3 (`AbilitySystemBlueprintLibrary.GetEffectContext` _returnvalue_2))
    (`GeneralBPFuncLibrary.EffectContextAddTargetData` _returnvalue_3 TargetData)
    (`self.K2_ExecuteGameplayCueWithParams` (struct :`TagName` "GameplayCue.Weapon.Scattergun.Fire") (`AbilitySystemBlueprintLibrary.MakeGameplayCueParameters` 0.0 0.0 _returnvalue_3))
    (else
      (`self.K2_CancelAbility`))))

(event `self.K2_OnEndAbility`
  (params (bWasCancelled :type Boolean))
  (bind _serverwaittargetdatatask (`self.ServerWaitTargetDataTask`))
  (`/Engine/EditorBlueprintResources/StandardMacros.IsValid` _serverwaittargetdatatask
    (:`Is Valid`
      (`GameplayTask.EndTask` _serverwaittargetdatatask))))