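; Base player controller that shows the team selection screen to remote clients once the game has started.
; On BeginPlay, the non-authority side checks FPSmthGameStateBase and either opens BP_UI_TeamSelection immediately or waits for its OnGameStarted event.
; The widget's OnUIFinish event triggers CloseCurrentWidget, which removes it and hides the mouse cursor.
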(event `self.ReceiveBeginPlay`
  (`/Engine/EditorBlueprintResources/ActorMacros.Switch Has Authority`
    (:`Remote`
      (bind _asfpsmth_game_state_base (cast `FPSmthGameStateBase` (`GameplayStatics.GetGameState`)))
      (if (`FPSmthGameStateBase.IsGameStarted` _asfpsmth_game_state_base)
        (bind _returnvalue (`|CreateWidget` "/Game/Blueprints/UI/BP_UI_TeamSelection.BP_UI_TeamSelection_C" self :!label _label))
        (bind _output_get (set `self.CurrentUIWidget` _returnvalue))
        (add `UserWidgetBase.OnUIFinish` _output_get (delegate `UserWidgetFinished`))
        (bind _returnvalue_2 (`UserWidget.AddToPlayerScreen` _output_get 0))
        (set `self.bShowMouseCursor` _returnvalue_2)
        (else
          (add `FPSmthGameStateBase.OnGameStarted` _asfpsmth_game_state_base (delegate `OnGameStarted_Event_0`)))))))

(event `UserWidgetFinished`
  (`self.CloseCurrentWidget`))

(event `OnGameStarted_Event_0`
  (goto _label))

(fn `UserConstructionScript`)