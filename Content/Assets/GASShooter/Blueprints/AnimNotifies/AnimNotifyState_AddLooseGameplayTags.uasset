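; Anim notify state that grants a set of loose gameplay tags to the animating character's ability system for the length of the notify window.
; On begin it casts the mesh owner, gets its ability system component and adds the configured GameplayTags with a count of one.
; On end it removes the same tags through the same lookup, and either event does nothing if a cast fails.
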(fn `Received_NotifyBegin`
  (params (MeshComp :type "SkeletalMeshComponent Object Reference") (Animation :type "AnimSequenceBase Object Reference") (TotalDuration :type "Float (double-precision)"))
  (returns (ReturnValue :type Boolean))
  (bind _asgscharacter_base (cast `` (`ActorComponent.GetOwner` MeshComp)))
  (bind _asgsability_system_component (cast `` (`AbilitySystemBlueprintLibrary.GetAbilitySystemComponent` _asgscharacter_base)))
  (`self.K2_AddLooseGameplayTags` _asgsability_system_component (`self.GameplayTags`) 1)
  (return true))

(fn `Received_NotifyEnd`
  (params (MeshComp :type "SkeletalMeshComponent Object Reference") (Animation :type "AnimSequenceBase Object Reference"))
  (returns (ReturnValue :type Boolean))
  (bind _asgscharacter_base (cast `` (`ActorComponent.GetOwner` MeshComp)))
  (bind _asgsability_system_component (cast `` (`AbilitySystemBlueprintLibrary.GetAbilitySystemComponent` _asgscharacter_base)))
  (`self.K2_RemoveLooseGameplayTags` _asgsability_system_component (`self.GameplayTags`) 1)
  (return true))