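; Gameplay ability that slows the owner's fall while input is held, by lowering the movement component's gravity scale.
; On activation it applies the slow-fall gameplay effect and cue, then loops short WaitDelay checks on IsFalling, re-creating a WaitInputRelease task each pass.
; Releasing input or no longer falling ends the ability, which removes the effect and sets gravity scale to a hard-coded default rather than the prior value.
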(event `self.K2_ActivateAbility`
  (set `self.EndThisAbility` false)
  (bind _returnvalue (`self.BP_ApplyGameplayEffectToOwner` "/Game/Characters/GASShared/GE_SlowFall_BP.GE_SlowFall_BP_C"))
  (set `self.GESlowFall` _returnvalue)
  (`self.K2_AddGameplayCue` (struct :`TagName` "GameplayCue.Player.SlowFall"))
  (bind _ascharacter_movement_component (cast `CharacterMovementComponent` (`.MovementComponent` (break `GameplayAbilityActorInfo` (`self.GetActorInfo`)))))
  (set `CharacterMovementComponent.GravityScale` 0.3 _ascharacter_movement_component)
  (`AbilityTask_WaitInputRelease.WaitInputRelease` false :!label _label
    (:`then`
      (`AbilityTask_WaitDelay.WaitDelay` 0.05
        (:`then`
          (bind _ascharacter_movement_component_2 (cast `CharacterMovementComponent` (`.MovementComponent` (break `GameplayAbilityActorInfo` (`self.GetActorInfo`)))))
          (if (`NavMovementComponent.IsFalling` _ascharacter_movement_component_2)
            (if (not (`self.EndThisAbility`))
              (goto _label))
            (else
              (set `self.EndThisAbility` true :!label _label_2)
              (`self.K2_EndAbility`))))))
    (:`OnRelease`
      (goto _label_2))))

(event `self.K2_OnEndAbility`
  (params (bWasCancelled :type Boolean))
  (`self.BP_RemoveGameplayEffectFromOwnerWithHandle` (`self.GESlowFall`))
  (bind _ascharacter_movement_component (cast `CharacterMovementComponent` (`.MovementComponent` (break `GameplayAbilityActorInfo` (`self.GetActorInfo`)))))
  (set `CharacterMovementComponent.GravityScale` 1.0 _ascharacter_movement_component))